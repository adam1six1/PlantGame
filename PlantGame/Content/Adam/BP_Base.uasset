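; BP_Base is a base structure that enemies attack, tracking its health from a starting maximum.
; On BeginPlay it binds to the BP_enemySpawn target-refresh event and, on each refresh, binds to every listed enemy1's attack event.
; Attacks targeting this actor subtract health, with no handling at zero.
; Tick pushes the health fraction to the BaseHealth bar in the first-person character's UI.
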(event Custom|receiveDamage
  (params (damage :type Float%20%28double-precision%29) (attackTarget :type Actor%20Object%20Reference))
  ;[1 1 1] receive damage
  (if (== attackTarget self)
    (Variables|Default|SetcurrentHealth (- (Variables|Default|GetcurrentHealth) damage))))

(event Custom|updateActors
  (params (plantsList :type Array%20of%20Actor%20Object%20References) (enemiesList :type Array%20of%20Actor%20Object%20References))
  ;[1 1 1] bind to other actors
  (bind _output_get (Variables|Default|SetEnemies%20List enemiesList))
  (for _array_element _output_get
    (EventDispatchers|BindEventtoOnEnemyAttack (.AsEnemy%201 (Utilities|Casting|CastToenemy1 _array_element)) (delegate Custom|receiveDamage))))

(event Custom|bindToSpawner
  ;[1 1 1] bind to other actors
  (bind _returnvalue (Actor|GetActorOfClass "/Game/Adam/enemySpawn/BP_enemySpawn.BP_enemySpawn_C"))
  (EventDispatchers|BindEventtoOnRefreshTargets _returnvalue (delegate Custom|updateActors)))

(event EventBeginPlay
  (Variables|Default|SetcurrentHealth (Variables|Default|GetmaxHealth))
  (CallFunction|BindtoSpawner))

(event Collision|EventActorBeginOverlap
  (params (OtherActor :type Actor%20Object%20Reference)))

(event EventTick
  (params (DeltaSeconds :type Float%20%28single-precision%29))
  (Progress|SetPercent (Variables|/Game/Widgets/WB_PlayerUI.WB_PlayerUI_C|GetbaseHealth (Variables|/Game/FirstPerson/Blueprints/BP_FirstPersonCharacter.BP_FirstPersonCharacter_C|GetplayerUI (.AsBP%20First%20Person%20Character (Utilities|Casting|CastToBP_FirstPersonCharacter (Game|GetPlayerCharacter 0))))) (/ (Variables|Default|GetcurrentHealth) (Variables|Default|GetmaxHealth))))

(fn ConstructionScript)