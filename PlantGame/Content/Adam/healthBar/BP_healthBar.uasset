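; BP_healthBar is a world-placed health bar actor that displays a HealthPercent value and always faces the player's camera.
; Each tick it casts its widget component's widget to WB_healthBar and sets that progress bar's percent from HealthPercent.
; It then rotates the whole actor toward the camera manager's location with a look-at rotation, acting as a billboard.
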(event EventBeginPlay)

(event Collision|EventActorBeginOverlap
  (params (OtherActor :type Actor%20Object%20Reference)))

(event EventTick
  (params (DeltaSeconds :type Float%20%28single-precision%29))
  ;[0.5 1 1] Sets health bar
  (bind _aswb_health_bar (Utilities|Casting|CastToWB_healthBar (UserInterface|GetWidget (Variables|Default|GetWidget))))
  (Progress|SetPercent (Variables|/Game/Adam/healthBar/WB_healthBar.WB_healthBar_C|GethealthBar _aswb_health_bar) (Variables|Default|GethealthPercent))
  ;[1 0.5 0.5] Rotate to camera
  (Transformation|SetActorRotation (Math|Rotator|FindLookatRotation (Transformation|GetActorLocation self) (Camera|GetCameraLocation (Game|GetPlayerCameraManager 0)))))

(fn ConstructionScript)