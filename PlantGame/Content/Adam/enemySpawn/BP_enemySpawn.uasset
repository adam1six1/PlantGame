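; Enemy spawner that periodically spawns an enemy on a circle's perimeter and tracks live plants and enemies for targeting.
; A Tick-driven countdown rotates and offsets the Spawner component to a random perimeter point, then spawns Enemy1 if the "enemy"-tag count is below the cap.
; Spawn and death dispatchers from the player, plants and enemies update both arrays, which are rebroadcast through OnRefreshTargets.
; The construction script scales SpawnRange to show the radius.
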(event Custom|updateTimer
  ;[1 1 1] Timer
  ;;[1 1 1] Increment timer
  (Variables|Default|Settimer (- (Variables|Default|Gettimer) (Variables|Default|GetdeltaTime)))
  ;;[1 1 1] Reset timer
  (if (<= (Variables|Default|Gettimer) 0.0)
    (Variables|Default|Settimer (Variables|Default|GetspawnRate))
    (CallFunction|SpawnLocation)
    (CallFunction|SpawnEnemy)))

(event Custom|spawnLocation
  ;[1 1 1] reset position
  (Transformation|SetRelativeLocation (Variables|Default|Getspawner) "0, 0, 0" false false)
  ;[1 1 1] random point on spawn range perimiter
  (Transformation|SetWorldRotation (Variables|Default|Getspawner) (Math|Rotator|MakeRotator 0.0 0.0 (* (Math|Random|RandomFloat) 3.6e+02)) false false)
  (Transformation|AddLocalOffset (Variables|Default|Getspawner) (Math|Vector|MakeVector 0.0 (Variables|Default|GetspawnRadius) 0.0) false false))

(event Custom|onPlantSpawn
  (params (plant :type Actor%20Object%20Reference))
  ;[1 1 1] event dispatchers
  (Utilities|Array|Add (Variables|Default|GetplantsArray) plant)
  (EventDispatchers|BindEventtoOnPlantDeath (.AsBP%20Base%20Plant (Utilities|Casting|CastToBP_basePlant plant)) (delegate Custom|onPlantDeath))
  (CallFunction|RefreshTargets))

(event Custom|onPlantDeath
  (params (deadPlant :type Actor%20Object%20Reference))
  ;[1 1 1] event dispatchers
  (Utilities|Array|RemoveItem (Variables|Default|GetplantsArray) deadPlant)
  (CallFunction|RefreshTargets))

(event Custom|enemyDead
  (params (deadEnemy :type Actor%20Object%20Reference))
  ;[1 1 1] event dispatchers
  (Utilities|Array|RemoveItem (Variables|Default|GetenemiesArray) deadEnemy)
  (CallFunction|RefreshTargets))

(event Custom|refreshTargets
  ;[1 1 1] event dispatchers
  (Default|CallOnRefreshTargets (Variables|Default|GetplantsArray) (Variables|Default|GetenemiesArray)))

(event Custom|spawnEnemy
  ;[1 1 1] check if enemy cap is hit
  (bind _outactors (Actor|GetAllActorswithTag "enemy"))
  (if (< (Utilities|Array|LastIndex _outactors) (+ (Variables|Default|GetmaxEnemies) -1))
    ;[1 1 1] spawn random enemy
    (bind _returnvalue (Game|SpawnActorfromClass "/Game/Adam/enemy1.enemy1_C" (Transformation|GetWorldTransform (Variables|Default|Getspawner)) "Undefined" "MultiplyWithRoot" 0 0))
    (Default|CallOnEnemySpawn _returnvalue)))

(event Custom|bindToPlayer
  ;[1 1 1] event dispatchers
  (EventDispatchers|BindEventtoOnPlantSpawn (.AsBP%20First%20Person%20Character (Utilities|Casting|CastToBP_FirstPersonCharacter (Game|GetPlayerCharacter 0))) (delegate Custom|onPlantSpawn))
  (EventDispatchers|BindEventtoOnEnemySpawn (delegate Custom|enemySpawned)))

(event Custom|enemySpawned
  (params (spawnedEnemy :type Actor%20Object%20Reference))
  ;[1 1 1] event dispatchers
  (Utilities|Array|Add (Variables|Default|GetenemiesArray) spawnedEnemy)
  (EventDispatchers|BindEventtoOnEnemyDeath (.AsEnemy%201 (Utilities|Casting|CastToenemy1 spawnedEnemy)) (delegate Custom|enemyDead))
  (CallFunction|RefreshTargets))

(event EventBeginPlay
  (Variables|Default|Settimer (Variables|Default|GetspawnRate))
  (CallFunction|BindtoPlayer))

(event Collision|EventActorBeginOverlap
  (params (OtherActor :type Actor%20Object%20Reference)))

(event EventTick
  (params (DeltaSeconds :type Float%20%28single-precision%29))
  (Variables|Default|SetdeltaTime DeltaSeconds)
  (CallFunction|UpdateTimer))

(fn ConstructionScript
  (bind _spawnradius (Variables|Default|GetspawnRadius))
  (bind _returnvalue (/ _spawnradius 5e+01))
  (Rendering|SetVisibility (Variables|Default|GetspawnRange) (Variables|Default|Getvisible) false)
  (Transformation|SetWorldScale3D (Variables|Default|GetspawnRange) (Math|Vector|MakeVector _returnvalue _returnvalue 1.0)))