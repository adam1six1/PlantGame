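; Base plant actor for a plant defense game, configured on BeginPlay from the player's selected slot as a default attacker, area-damage rosebush or high-health, no-damage hedge.
; Each Tick updates health, checks range and line of sight to the nearest enemy, rotates and attacks on a cooldown.
; Damage passes both ways through event dispatchers, with target lists refreshed by the enemy spawner and death broadcast before destruction.
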(event OnComponentBeginOverlap(sphereHitbox)
  (params (OverlappedComponent :type Primitive%20Component%20Object%20Reference) (OtherActor :type Actor%20Object%20Reference) (OtherComp :type Primitive%20Component%20Object%20Reference) (OtherBodyIndex :type Integer) (bFromSweep :type Boolean) (SweepResult :type Hit%20Result%20Structure%20%28by%20ref%29))
  ;[1 1 1] switch target when attacked
)

(event Custom|bind%20to%20enemySpawn
  ;[1 1 1] bind to enemy spawn
  (bind _returnvalue (Actor|GetActorOfClass "/Game/Adam/enemySpawn/BP_enemySpawn.BP_enemySpawn_C"))
  (EventDispatchers|BindEventtoOnRefreshTargets _returnvalue (delegate Custom|updateActors)))

(event Custom|plantHealth
  (bind _helthbar (Variables|Default|GethelthBar))
  ;[1 1 1] Health
  ;;[1 0.5 0.5] Destroy when no health
  (if (<= (Variables|Default|GetcurrentHealth) 0)
    (Default|CallOnPlantDeath self)
    (Actor|DestroyActor)
    (else
      ;;[0.5 1 1] Set healthbar
      (Default|UpdateHealthbar (.AsWB%20Health%20Bar (Utilities|Casting|CastToWB_healthBar (UserInterface|GetWidget _helthbar))) (Variables|Default|GetcurrentHealth) (Variables|Default|GetmaxHealth) _helthbar))))

(event Custom|roseBushAttack
  (bind _rosebushattackrange (Variables|Default|GetrosebushAttackRange))
  (bind _range (Variables|Default|Getrange))
  (bind _returnvalue (/ _range 5e+01))
  ;[1 1 1] rosebush
  (if (< (.Distance (Actor|FindNearestActor (Transformation|GetActorLocation) (Variables|Default|GetenemiesArray))) (Variables|Default|Getrange))
    (Utilities|Array|Clear (Variables|Default|GetroseBushTargets))
    (Variables|Default|Settimer 0.0)
    (for _array_element (Variables|Default|GetenemiesArray)
      (if (< (Transformation|GetDistanceTo _array_element) (Variables|Default|Getrange))
        (Default|CallOnPlantAttack (Variables|Default|Getdamage) _array_element)))
    (Transformation|SetWorldScale3D _rosebushattackrange (Math|Vector|MakeVector _returnvalue _returnvalue (.z (Transformation|GetWorldScale (Variables|Default|GetrosebushAttackRange)))))
    (Rendering|SetVisibility _rosebushattackrange true false)
    (Utilities|FlowControl|Delay 0.2)
    (Rendering|SetVisibility _rosebushattackrange false false)))

(event Custom|updateActors
  (params (plantsList :type Array%20of%20Actor%20Object%20References) (enemiesList :type Array%20of%20Actor%20Object%20References))
  ;[1 1 1] bind to enemy spawn
  (Variables|Default|SetplantsArray plantsList)
  (Variables|Default|SetenemiesArray enemiesList)
  (CallFunction|RefreshTarget))

(event Custom|hedgeSetup
  (bind _plantmesh (Variables|Default|GetplantMesh))
  ;[1 1 1] hedge
  (bind _output_get (Variables|Default|SetmaxHealth 1.5e+02))
  (Variables|Default|SetcurrentHealth _output_get)
  (Variables|Default|Setdamage 0.0)
  (Components|StaticMesh|SetStaticMesh _plantmesh "/Game/Assets/plantModels/hedge_1_.hedge_1_")
  (Rendering|Material|SetMaterial _plantmesh 0 "/Game/Assets/plantModels/M_hedge.M_hedge")
  (Variables|Default|SetcanRotate? false))

(event Custom|bindToEnemyAttack
  ;[1 1 1] Bind to enemy attack
  (for _array_element (Variables|Default|GetenemiesArray)
    (EventDispatchers|BindEventtoOnEnemyAttack (.AsEnemy%201 (Utilities|Casting|CastToenemy1 _array_element)) (delegate Custom|reciveDamage))))

(event Custom|reciveDamage
  (params (damage :type Float%20%28double-precision%29) (attackTarget :type Actor%20Object%20Reference))
  ;[1 1 1] recive damage
  (if (== attackTarget self)
    (Variables|Default|SetcurrentHealth (- (Variables|Default|GetcurrentHealth) damage))))

(event Custom|setTarget
  ;[1 1 1] set nearest target
)

(event Custom|rotateToTarget
  ;[1 1 1] rotate to target
  (if (and (Variables|Default|GetenemyInRange?) (Variables|Default|GetcanRotate?))
    (Transformation|SetActorRotation (Math|Rotator|MakeRotator 0.0 0.0 (.yaw (Math|Rotator|FindLookatRotation (Transformation|GetActorLocation) (Transformation|GetActorLocation (Variables|Default|GetcurrentTarget))))))))

(event Custom|attack
  ;[1 1 1] attack
  (if (Variables|Default|GetisRosebush?)
    (CallFunction|RoseBushAttack)
    (elif (Variables|Default|GetenemyInRange?)
      (Variables|Default|Settimer 0.0)
      (Default|CallOnPlantAttack (Variables|Default|Getdamage) (Variables|Default|GetcurrentTarget)))))

(event Custom|attackCooldown
  ;[1 1 1] attack cooldown
  (if (< (Variables|Default|Gettimer) (Variables|Default|GetattackSpeed))
    (Variables|Default|Settimer (+ (Variables|Default|GetDelta%20Seconds) (Variables|Default|Gettimer)))
    (else
      (CallFunction|Attack))))

(event Custom|getPlantType
  ;[1 1 1] get plant type
  (bind _output_get (Variables|Default|SetplantNum (Variables|/Game/FirstPerson/Blueprints/BP_FirstPersonCharacter.BP_FirstPersonCharacter_C|GetCurr%20Slot (.AsBP%20First%20Person%20Character (Utilities|Casting|CastToBP_FirstPersonCharacter (Game|GetPlayerCharacter 0))))))
  (switch int _output_get
    (:Default
      (Rendering|SetVisibility (Variables|Default|Getneck) true true))
    (:1
      (CallFunction|RoseBushSetup))
    (:2
      (CallFunction|HedgeSetup))))

(event Custom|roseBushSetup
  (bind _plantmesh (Variables|Default|GetplantMesh))
  ;[1 1 1] rosebush
  (bind _output_get (Variables|Default|SetmaxHealth 7e+01))
  (Variables|Default|SetcurrentHealth _output_get)
  (Variables|Default|Setdamage 1e+01)
  (Variables|Default|SetattackSpeed 0.5)
  (Variables|Default|Setrange 5e+02)
  (Variables|Default|SetisRosebush? true)
  (Components|StaticMesh|SetStaticMesh _plantmesh "/Game/Assets/plantModels/rosebush_1_.rosebush_1_")
  (Rendering|Material|SetMaterial _plantmesh 0 "/Game/Assets/plantModels/M_rosebush.M_rosebush")
  (Variables|Default|SetcanRotate? false))

(event Custom|refreshTarget
  ;[1 1 1] refreshTarget
  (CallFunction|BindtoEnemyAttack)
  (Variables|Default|SetcurrentTarget (.ReturnValue (Actor|FindNearestActor (Transformation|GetActorLocation) (Variables|Default|GetenemiesArray)))))

(event Custom|enemyWithinRange
  ;[1 1 1] enemy within range?
  (bind _currenttarget (Variables|Default|GetcurrentTarget)
    (:then
      (bind _output_get (Variables|Default|SetactorsToIgnore (Variables|Default|GetplantsArray)))
      (Utilities|Array|Add _output_get (Game|GetPlayerController 0))
      (bind _returnvalue (Collision|LineTraceByChannel (+ (Transformation|GetActorLocation) "0.000000,0.000000,100.000000") (+ (Transformation|GetActorLocation _currenttarget) "0.000000,0.000000,100.000000") "TraceTypeQuery1" false (Variables|Default|GetactorsToIgnore) "None"))
      (Variables|Default|SetenemyInRange? (and _returnvalue (< (Math|Vector|Distance(Vector) (Transformation|GetActorLocation _currenttarget) (Transformation|GetActorLocation)) (Variables|Default|Getrange)))))
    (:else
      (Variables|Default|SetenemyInRange? false))))

(event EventBeginPlay
  (bind _outactors (Actor|GetAllActorsOfClass "/Game/Adam/enemy1.enemy1_C"))
  (Variables|Default|SetenemiesArray _outactors)
  (CallFunction|BindtoEnemySpawn)
  (CallFunction|RefreshTarget)
  (CallFunction|GetPlantType))

(event Collision|EventActorBeginOverlap
  (params (OtherActor :type Actor%20Object%20Reference)))

(event EventTick
  (params (DeltaSeconds :type Float%20%28single-precision%29))
  (Variables|Default|SetDelta%20Seconds DeltaSeconds)
  (CallFunction|PlantHealth)
  (CallFunction|EnemyWithinRange)
  (CallFunction|AttackCooldown)
  (CallFunction|RotatetoTarget))

(fn ConstructionScript)