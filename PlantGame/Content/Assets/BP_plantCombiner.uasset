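; Plant combiner machine that merges two seeds from the player's Hotbar into a new seed type.
; Player interact events on its collision components deposit or return input seeds, collect the output, or trigger combining.
; Widget brushes double as slot state, with MysteryPlant meaning empty and seed image lookups giving the index.
; Combining concatenates both seeds' PlantStrings in index order, making recipes order-independent, and a matching entry becomes the output seed.
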(event Custom|playerInteract
  (params (hitComponent :type String))
  (switch string hitComponent
    (:BP_plantCombiner.input1
      (CallFunction|InputButton (Variables|Default|Getimage1))
      (Default|CallSeedAmountChanged (Variables|Default|GetHotbar) :!label _label))
    (:BP_plantCombiner.input2
      (CallFunction|InputButton (Variables|Default|Getimage2))
      (goto _label))
    (:BP_plantCombiner.output
      (CallFunction|OutputButton)
      (goto _label))
    (:BP_plantCombiner.buttonCollision
      (CallFunction|ButtonPushed))))

(event Custom|inputButton
  (params (image :type Widget%20Component%20Object%20Reference))
  (bind _returnvalue (UserInterface|GetWidget image))
  (bind _hotbar (Variables|Default|GetHotbar))
  (bind _hotbar_2 (Variables|Default|GetHotbar))
  (bind _hotbar_3 (Variables|Default|GetHotbar))
  (bind _aswb_plant_combiner (Utilities|Casting|CastToWB_plantCombiner _returnvalue))
  (bind _plantseedimages (Variables|/Game/Widgets/WB_hotbar.WB_hotbar_C|GetplantSeedImages _hotbar_2))
  (bind _currentslot (Variables|/Game/Widgets/WB_hotbar.WB_hotbar_C|GetcurrentSlot _hotbar_3))
  (bind _brush (Variables|/Script/UMG.Image|GetBrush (Variables|/Game/Widgets/WB_plantCombiner.WB_plantCombiner_C|Getimage _aswb_plant_combiner)))
  (bind _returnvalue_2 (Utilities|Array|FindItem _plantseedimages _brush))
  (if (== _brush (Variables|Default|GetmysteryPlant))
    (if (> (Utilities|Array|Get(acopy) (Variables|/Game/Widgets/WB_hotbar.WB_hotbar_C|GetseedAmount _hotbar) (Variables|/Game/Widgets/WB_hotbar.WB_hotbar_C|GetcurrentSlot _hotbar)) 0)
      (Class|Image|SetBrush (Variables|/Game/Widgets/WB_plantCombiner.WB_plantCombiner_C|Getimage _aswb_plant_combiner) (Utilities|Array|Get(acopy) (Variables|/Game/Widgets/WB_hotbar.WB_hotbar_C|GetplantSeedImages _hotbar_3) _currentslot))
      (Math|Integer|DecrementInt (Utilities|Array|Get(acopy) (Variables|/Game/Widgets/WB_hotbar.WB_hotbar_C|GetseedAmount _hotbar_3) _currentslot)))
    (else
      (if (!= _returnvalue_2 -1)
        (Math|Integer|IncrementInt (Utilities|Array|Get(acopy) (Variables|/Game/Widgets/WB_hotbar.WB_hotbar_C|GetseedAmount _hotbar_2) _returnvalue_2)
          (:%20%20
            _)))
      (Class|Image|SetBrush (Variables|/Game/Widgets/WB_plantCombiner.WB_plantCombiner_C|Getimage _aswb_plant_combiner) (Variables|Default|GetmysteryPlant)))))

(event Custom|buttonPushed
  (bind _imagebrushes (Variables|Default|GetimageBrushes))
  (bind _hotbar (Variables|Default|GetHotbar))
  (bind _plantstrings (Variables|Default|GetplantStrings))
  (bind _imagebrushes_2 (Variables|Default|GetimageBrushes))
  (bind _hotbar_2 (Variables|Default|GetHotbar))
  (bind _plantstrings_2 (Variables|Default|GetplantStrings))
  (bind _plantstrings_3 (Variables|Default|GetplantStrings))
  (bind _plantstrings_4 (Variables|Default|GetplantStrings))
  (bind _output (Utilities|Array|Get(acopy) _imagebrushes 1))
  (bind _output_2 (Utilities|Array|Get(acopy) _imagebrushes_2))
  (bind _plantseedimages (Variables|/Game/Widgets/WB_hotbar.WB_hotbar_C|GetplantSeedImages _hotbar))
  (bind _plantseedimages_2 (Variables|/Game/Widgets/WB_hotbar.WB_hotbar_C|GetplantSeedImages _hotbar_2))
  (bind _returnvalue (Utilities|Array|FindItem _plantseedimages _output))
  (bind _returnvalue_2 (Utilities|Array|FindItem _plantseedimages_2 _output_2))
  (bind _output_3 (Utilities|Array|Get(acopy) _plantstrings_2 _returnvalue_2))
  (bind _output_4 (Utilities|Array|Get(acopy) _plantstrings _returnvalue))
  (bind _returnvalue_3 (Utilities|String|Append _output_4 _output_3))
  (bind _returnvalue_4 (Utilities|String|Append _output_3 _output_4))
  (bind _returnvalue_5 (Utilities|Array|FindItem _plantstrings_3 _returnvalue_3))
  (bind _returnvalue_6 (Utilities|Array|FindItem _plantstrings_4 _returnvalue_4))
  (for (_array_element _array_index) (Utilities|Array|MakeArray (Variables|Default|Getimage1) (Variables|Default|Getimage2) (Variables|Default|Getimage3))
    (Utilities|Array|SetArrayElem (Variables|Default|GetimageBrushes) _array_index (Variables|/Script/UMG.Image|GetBrush (Variables|/Game/Widgets/WB_plantCombiner.WB_plantCombiner_C|Getimage (.AsWB%20Plant%20Combiner (Utilities|Casting|CastToWB_plantCombiner (UserInterface|GetWidget _array_element)))))))
  (if (Math|Boolean|ANDBoolean (not (== (Utilities|Array|Get(acopy) (Variables|Default|GetimageBrushes)) (Variables|Default|GetmysteryPlant))) (not (== (Utilities|Array|Get(acopy) (Variables|Default|GetimageBrushes) 1) (Variables|Default|GetmysteryPlant))) (== (Utilities|Array|Get(acopy) (Variables|Default|GetimageBrushes) 2) (Variables|Default|GetmysteryPlant)) (not (Variables|Default|GetoutputAvalable?)))
    (if (< _returnvalue_2 _returnvalue)
      (if (!= _returnvalue_6 -1)
        (Variables|Default|SetoutputSeed _returnvalue_6)
        (Class|Image|SetBrush (Variables|/Game/Widgets/WB_plantCombiner.WB_plantCombiner_C|Getimage (.AsWB%20Plant%20Combiner (Utilities|Casting|CastToWB_plantCombiner (UserInterface|GetWidget (Variables|Default|Getimage3))))) (Utilities|Array|Get(acopy) (Variables|/Game/Widgets/WB_hotbar.WB_hotbar_C|GetplantSeedImages (Variables|Default|GetHotbar)) (Variables|Default|GetoutputSeed)) :!label _label)
        (Variables|Default|SetoutputAvalable? true)
        (Class|Image|SetBrush (Variables|/Game/Widgets/WB_plantCombiner.WB_plantCombiner_C|Getimage (.AsWB%20Plant%20Combiner (Utilities|Casting|CastToWB_plantCombiner (UserInterface|GetWidget (Variables|Default|Getimage2))))) (Variables|Default|GetmysteryPlant)))
      (elif (!= _returnvalue_5 -1)
        (Variables|Default|SetoutputSeed _returnvalue_5)
        (goto _label)))))

(event Custom|outputButton
  (if (Variables|Default|GetoutputAvalable?)
    (Math|Integer|IncrementInt (Utilities|Array|Get(acopy) (Variables|/Game/Widgets/WB_hotbar.WB_hotbar_C|GetseedAmount (Variables|Default|GetHotbar)) (Variables|Default|GetoutputSeed))
      (:%20%20
        (Variables|Default|SetoutputAvalable? false)
        (Class|Image|SetBrush (Variables|/Game/Widgets/WB_plantCombiner.WB_plantCombiner_C|Getimage (.AsWB%20Plant%20Combiner (Utilities|Casting|CastToWB_plantCombiner (UserInterface|GetWidget (Variables|Default|Getimage3))))) (Variables|Default|GetmysteryPlant))))))

(event EventBeginPlay
  (bind _returnvalue (Game|GetPlayerCharacter 0))
  (bind _asbp_first_person_character (Utilities|Casting|CastToBP_FirstPersonCharacter _returnvalue))
  (EventDispatchers|BindEventtoOnPCInteract _asbp_first_person_character (delegate Custom|playerInteract))
  (Utilities|FlowControl|DelayUntilNextTick)
  (Variables|Default|SetHotbar (Variables|/Game/FirstPerson/Blueprints/BP_FirstPersonCharacter.BP_FirstPersonCharacter_C|Gethotbar _asbp_first_person_character)))

(event Collision|EventActorBeginOverlap
  (params (OtherActor :type Actor%20Object%20Reference)))

(event EventTick
  (params (DeltaSeconds :type Float%20%28single-precision%29)))

(fn ConstructionScript)