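; BP_Bed is a bed Blueprint that runs the in-game clock, with no sleep logic in its graphs.
; Tick accumulates real seconds, adding ten in-game minutes every 1.25 seconds, rolling over hours and midnight.
; Every tick it writes the hour:minute text to the first-person character's PlayerUI.
; The day counter is touched only in BeginPlay and never increments; DisplayDay and overlap events are empty.
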(event Custom|displayTime
  (Variables|/Script/UMG.TextBlock|SetText (Variables|/Game/Widgets/WB_PlayerUI.WB_PlayerUI_C|GetTime (Variables|/Game/FirstPerson/Blueprints/BP_FirstPersonCharacter.BP_FirstPersonCharacter_C|GetplayerUI (.AsBP%20First%20Person%20Character (Utilities|Casting|CastToBP_FirstPersonCharacter (Game|GetPlayerCharacter 0))))) (Utilities|Text|ToText(String) (Utilities|String|Append (Utilities|String|ToString(Integer) (Math|Float|Truncate (Variables|Default|GetingameHour))) ":" (Utilities|String|ToString(Integer) (Math|Float|Truncate (Variables|Default|GetingameMinutes)))))))

(event Custom|DisplayDay)

(event EventBeginPlay
  (Variables|Default|SetDayCounter (+ 0.0 (Variables|Default|GetDayCounter)))
  (if (>= (Variables|Default|GetingameHour) 24.0)
    (Variables|Default|SetDayCounter 0.0)))

(event Collision|EventActorBeginOverlap
  (params (OtherActor :type Actor%20Object%20Reference)))

(event EventTick
  (params (DeltaSeconds :type Float%20%28single-precision%29))
  (Variables|Default|SetrealSeconds (+ (Variables|Default|GetrealSeconds) DeltaSeconds))
  (CallFunction|DisplayTime)
  (if (> (Variables|Default|GetrealSeconds) 1.25)
    (Variables|Default|SetingameMinutes (+ (Variables|Default|GetingameMinutes) 1e+01))
    (Variables|Default|SetrealSeconds 0.0)
    (if (== (Variables|Default|GetingameMinutes) 6e+01)
      (Variables|Default|SetingameMinutes 0.0)
      (Variables|Default|SetingameHour (+ (Variables|Default|GetingameHour) 1.0))
      (if (>= (Variables|Default|GetingameHour) 24.0)
        (Variables|Default|SetingameHour 0.0)))))

(fn ConstructionScript)